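; BP_FPPT_PowerCube is a power cube actor that reports its power type and active state through GetActivatorPowerType.
; Pickup, Drop, material setup and Hit events are empty, while BeginPlay and the construction script only call the parent.
; Logic for motion-controller attach and detach with physics toggling, material assignment and speed-scaled bump sounds remains in the graph but is disconnected and never runs.
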(event `/Game/VirtualRealityBP/Blueprints/PickupActorInterface.Pickup`
  (params (AttachTo :type "SceneComponent Object Reference")))

(event `self.ReceiveBeginPlay`
  (`parent.ReceiveBeginPlay`))

(event `/Game/VirtualRealityBP/Blueprints/PickupActorInterface.Drop`)

(event `self.Setup Material Owners`)

(event `self.ReceiveHit`
  (params (MyComp :type "PrimitiveComponent Object Reference") (Other :type "Actor Object Reference") (OtherComp :type "PrimitiveComponent Object Reference") (bSelfMoved :type Boolean) (HitLocation :type "Vector Structure") (HitNormal :type "Vector Structure") (NormalImpulse :type "Vector Structure") (Hit :type "HitResult Structure (by ref)"))
  ;[1 1 1] Collision Sounds
)

(fn `Get Activator Power Type`
  (returns (`Power Type` :type "/Game/ProjectEternity/PuzzleBPs/structs/Enum_FPPT_Colors Enum") (`Is Active` :type Boolean))
  (return (`self.Power Type`) (`self.Active`)))

(fn `UserConstructionScript`
  (`parent.UserConstructionScript`))